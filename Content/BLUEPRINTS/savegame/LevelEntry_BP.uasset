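; Level entry portal actor that shows whether a quest is unlocked and opens that quest's level when the player walks into it.
; IsQuestUnlocked compares the player save data's highest unlocked quest against this portal's number.
; On BeginPlay an unlocked portal gets a metallic base and reveals its spinning quest icon, while a locked one turns red.
; Sphere overlap by the 731 character rechecks the unlock before loading the level.
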(event `self.ReceiveTick`
  (params (DeltaSeconds :type "Float (single-precision)"))
  (`SceneComponent.K2_AddRelativeRotation` (`self.Quest`) (struct :`Yaw` 1.0) false false))

(event `self.ReceiveBeginPlay`
  (bind _base (`self.Base`))
  (bind _returnvalue (`self.IsQuestUnlocked`))
  ;[1 1 1] If Quest is unlocked the base will be green and you will see a rotating quest icon
  (if _returnvalue
    (`PrimitiveComponent.SetMaterial` _base 0 "/Game/BLUEPRINTS/Materials/M_731base_Metalic.M_731base_Metalic")
    (`SceneComponent.SetHiddenInGame` (`self.Quest`) false false)
    (else
      (`PrimitiveComponent.SetMaterial` _base 0 "/Game/BLUEPRINTS/Materials/M_BasicColourRed.M_BasicColourRed"))))

(event `self.Sphere.OnComponentBeginOverlap`
  (params (OverlappedComponent :type "PrimitiveComponent Object Reference") (OtherActor :type "Actor Object Reference") (OtherComp :type "PrimitiveComponent Object Reference") (OtherBodyIndex :type Integer) (bFromSweep :type Boolean) (SweepResult :type "HitResult Structure (by ref)"))
  (cast `/Game/BLUEPRINTS/731Character` OtherActor)
  (bind _returnvalue (`self.IsQuestUnlocked`))
  (if _returnvalue
    (`GameplayStatics.OpenLevel` (`self.QuestToOpen`))))

(fn `IsQuestUnlocked`
  (returns (ReturnValue :type Boolean))
  (bind _playerstats (`/Game/BLUEPRINTS/731Character.GetCurrentPlayerSaveData` (`self.As 731Character`)))
  (return (>= (`.HighestQuestUnlocked_16_C457FA824C6C81C27ED51A95B13559F9` (break `/Game/BLUEPRINTS/savegame/PlayerStats_S` _playerstats)) (`self.PortalNumber`))))

(fn `UserConstructionScript`)