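; Quest giver actor that walks the player through dialogue, then opens a whiteboard of its quests.
; An overlap radius shows a camera-facing interaction prompt while the Quest component spins on Tick.
; Each Interact advances the dialogue widget; after the last line, the whiteboard widget is filled from the Quests array.
; Closing the board, by Interact or CloseQuestWidget, restores game-only input and destroys the actor.
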(event `self.ReceiveTick`
  (params (DeltaSeconds :type "Float (single-precision)"))
  (`|ExecutionSequence`
    (:`then_0`
      (`SceneComponent.K2_AddRelativeRotation` (`self.Quest`) (struct :`Yaw` 1.0) false false))
    (:`then_1`
      (`SceneComponent.K2_SetWorldRotation` (`self.InteractionPrompt`) (`KismetMathLibrary.FindLookAtRotation` (`SceneComponent.K2_GetComponentLocation` (`self.InteractionPrompt`)) (`SceneComponent.K2_GetComponentLocation` (`PlayerCameraManager.TransformComponent` (`GameplayStatics.GetPlayerCameraManager` 0)))) false false))))

(event `self.AcceptanceRadius.OnComponentBeginOverlap`
  (params (OverlappedComponent :type "PrimitiveComponent Object Reference") (OtherActor :type "Actor Object Reference") (OtherComp :type "PrimitiveComponent Object Reference") (OtherBodyIndex :type Integer) (bFromSweep :type Boolean) (SweepResult :type "HitResult Structure (by ref)"))
  (cast `/Game/BLUEPRINTS/731Character` OtherActor)
  (`SceneComponent.SetVisibility` (`self.InteractionPrompt`) true false))

(event `self.AcceptanceRadius.OnComponentEndOverlap`
  (params (OverlappedComponent :type "PrimitiveComponent Object Reference") (OtherActor :type "Actor Object Reference") (OtherComp :type "PrimitiveComponent Object Reference") (OtherBodyIndex :type Integer))
  (cast `/Game/BLUEPRINTS/731Character` OtherActor)
  (`SceneComponent.SetVisibility` (`self.InteractionPrompt`) false false))

(event `/Game/BLUEPRINTS/savegame/QuestSystem/QuestGiver_BPI.Interact`
  (bind _returnvalue (`GameplayStatics.GetPlayerController` 0))
  (bind _returnvalue_2 (`GameplayStatics.GetPlayerController` 0))
  (if (not (`self.IsBoardActive?`))
    ;[1 1 1] Changes dialogue each time you interact [E]
    (if (not (`self.DialogueOpen`))
      ;[1 1 1] Opens the quest dialogue widget
      (bind _returnvalue_3 (`|CreateWidget` "/Game/BLUEPRINTS/UI/QuestDialogue_WB.QuestDialogue_WB_C"))
      (set `self.DialogueREF` _returnvalue_3)
      (`UserWidget.AddToViewport` _returnvalue_3 0)
      (set `self.DialogueOpen` true)
      (`TextBlock.SetText` (`/Game/BLUEPRINTS/UI/QuestDialogue_WB.Dialogue` (`self.DialogueREF`)) (`KismetTextLibrary.Conv_StringToText` (`|GetArrayItem` (`self.Dialogue`) (`self.DialogueIndex`))))
      (`/Engine/EditorBlueprintResources/StandardMacros.IncrementInt` (`self.DialogueIndex`)
        (:`  `
          (set `PlayerController.bShowMouseCursor` true _returnvalue_2)
          (`WidgetBlueprintLibrary.SetInputMode_GameAndUIEx` _returnvalue_2 (`self.QuestWhiteboardREF`))))
      (else
        (`TextBlock.SetText` (`/Game/BLUEPRINTS/UI/QuestDialogue_WB.Dialogue` (`self.DialogueREF`)) (`KismetTextLibrary.Conv_StringToText` (`|GetArrayItem` (`self.Dialogue`) (`self.DialogueIndex`))))
        (`/Engine/EditorBlueprintResources/StandardMacros.IncrementInt` (`self.DialogueIndex`)
          (:`  `
            (if (> (`self.DialogueIndex`) (`KismetArrayLibrary.Array_Length` (`self.Dialogue`)))
              (`Widget.RemoveFromParent` (`self.DialogueREF`))
              (set `self.DialogueREF` null)
              (set `self.DialogueIndex` 0)
              (set `self.DialogueOpen` false)
              (`self.OpenQuestWB`))))))
    (else
      (`Widget.RemoveFromParent` (`self.QuestWhiteboardREF`) :!label _label)
      (set `self.QuestWhiteboardREF` null)
      (set `PlayerController.bShowMouseCursor` false _returnvalue)
      (`WidgetBlueprintLibrary.SetInputMode_GameOnly` _returnvalue)
      (set `self.IsBoardActive?` false)
      ;[1 1 1] Quest giver has been destroyed here
      (`self.K2_DestroyActor`))))

(event `OpenQuestWB`
  ;[1 1 1] If Whiteboard is not active create one
  (bind _returnvalue (`|CreateWidget` "/Game/BLUEPRINTS/UI/QuestWhiteboard_WB.QuestWhiteboard_WB_C"))
  (bind _output_get (set `self.QuestWhiteboardREF` _returnvalue))
  (`UserWidget.AddToViewport` _output_get 0)
  (set `self.IsBoardActive?` true)
  (set `/Game/BLUEPRINTS/UI/QuestWhiteboard_WB.WhiteBoard_BP` self (`self.QuestWhiteboardREF`))
  (for _array_element (`self.Quests`)
    (`/Game/BLUEPRINTS/UI/QuestWhiteboard_WB.AddNewQuest` (`self.QuestWhiteboardREF`) _array_element)))

(event `CloseQuestWidget`
  (goto _label))

(fn `UserConstructionScript`)