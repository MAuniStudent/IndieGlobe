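; Quest component that tracks the active quest's objectives and updates the player character's HUD.
; CollectOrEndActors removes reported actors from a temporary copy of an objective's actor list, completing it when empty, while OpenRewardChest completes objectives with a matching reward chest.
; Each completion increments a counter in ObjectiveCompleted.
; When all objectives are done, it clears the quest, briefly shows the completion widget, hides quest UI and sets QuestCompleted.
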(event `self.ReceiveBeginPlay`
  (bind _as731character (cast `/Game/BLUEPRINTS/731Character` (`GameplayStatics.GetPlayerCharacter` 0)))
  (set `self.As 731Character` _as731character))

(event `SetActiveQuestText`
  (bind _activequest_wb (`/Game/BLUEPRINTS/UI/PlayerHUD.ActiveQuest_WB` (`/Game/BLUEPRINTS/731Character.PlayerHUDref` (`self.As 731Character`))))
  (`Widget.SetVisibility` _activequest_wb "Visible")
  (`TextBlock.SetText` (`/Game/BLUEPRINTS/UI/ActiveQuest_WB.CurrentQuest` _activequest_wb) (`KismetTextLibrary.Conv_StringToText` (`.QuestName_3_3AC3368347468032314BE0A0D82DB1D1` (break `/Game/BLUEPRINTS/savegame/QuestSystem/Quests_S` (`self.ActiveQuest`))))))

(event `SetObjectives`
  (bind (_activequest_questname _activequest_description _activequest_hassecondary _activequest_iscompleted _activequest_questobjectives) (break `/Game/BLUEPRINTS/savegame/QuestSystem/Quests_S` (`self.ActiveQuest`)))
  (`/Game/BLUEPRINTS/UI/PlayerHUD.PopulateObjectives` (`/Game/BLUEPRINTS/731Character.PlayerHUDref` (`self.As 731Character`)) _activequest_questobjectives))

(event `CollectOrEndActors`
  (params (Actor :type "Actor Object Reference"))
  (bind (_activequest_questname _activequest_description _activequest_hassecondary _activequest_iscompleted _activequest_questobjectives) (break `/Game/BLUEPRINTS/savegame/QuestSystem/Quests_S` (`self.ActiveQuest`)))
  (bind _returnvalue (`KismetArrayLibrary.Array_Length` (`self.TempActorArray`)))
  (for _array_element _activequest_questobjectives
    (bind (_name _completed _collectorendactors _chestreward _ispickedupordestroyed _isrewardavailable_) (break `/Game/BLUEPRINTS/savegame/QuestSystem/QuestObjectives_S` _array_element))
    ;[1 1 1] Temparary Array used to eliminate actors from a specific quest objective in order to complete the tast
    (if (and (not _completed) _ispickedupordestroyed)
      (if (not (!= (`KismetArrayLibrary.Array_Length` (`self.TempActorArray`)) 0))
        (bind _output_get (set `self.TempActorArray` _collectorendactors)))
      (`KismetArrayLibrary.Array_RemoveItem` _output_get Actor)
      (`|VariableSetRef` _array_element (make `/Game/BLUEPRINTS/savegame/QuestSystem/QuestObjectives_S` _name false (`self.TempActorArray`) _chestreward false _isrewardavailable_))
      ;;[0.4859 0.03574 0] Only For Debugging
      (`KismetSystemLibrary.PrintString` (`KismetStringLibrary.Conv_IntToString` _returnvalue))
      (if (== _returnvalue 0)
        (`|VariableSetRef` _array_element (make `/Game/BLUEPRINTS/savegame/QuestSystem/QuestObjectives_S` _name true _ _chestreward false _isrewardavailable_))
        ;[1 1 1] Quest completed when objectives are met
        (`/Game/BLUEPRINTS/UI/PlayerHUD.CompleteObjectives` (`/Game/BLUEPRINTS/731Character.PlayerHUDref` (`self.As 731Character`)) _array_element)
        (`self.ObjectiveCompleted`)
        ;[0.4859 0.03574 0] Only for Debugging
        (`KismetSystemLibrary.PrintString` "COMPLETED")))))

(event `OpenRewardChest`
  (params (ChestReward :type "Actor Object Reference"))
  (bind (_activequest_questname _activequest_description _activequest_hassecondary _activequest_iscompleted _activequest_questobjectives) (break `/Game/BLUEPRINTS/savegame/QuestSystem/Quests_S` (`self.ActiveQuest`)))
  (for _array_element _activequest_questobjectives
    (bind (_name _completed _collectorendactors _chestreward _ispickedupordestroyed _isrewardavailable_) (break `/Game/BLUEPRINTS/savegame/QuestSystem/QuestObjectives_S` _array_element))
    (if (and _isrewardavailable_ (== ChestReward _chestreward))
      (`|VariableSetRef` _array_element (make `/Game/BLUEPRINTS/savegame/QuestSystem/QuestObjectives_S` _name true _collectorendactors null _ispickedupordestroyed _isrewardavailable_))
      ;[1 1 1] Quest completed when objectives are met
      (`/Game/BLUEPRINTS/UI/PlayerHUD.CompleteObjectives` (`/Game/BLUEPRINTS/731Character.PlayerHUDref` (`self.As 731Character`)) _array_element)
      (`self.ObjectiveCompleted`))))

(event `ObjectiveCompleted`
  (bind (_activequest_questname _activequest_description _activequest_hassecondary _activequest_iscompleted _activequest_questobjectives) (break `/Game/BLUEPRINTS/savegame/QuestSystem/Quests_S` (`self.ActiveQuest`)))
  (`/Engine/EditorBlueprintResources/StandardMacros.IncrementInt` (`self.CompletedObjective`)
    (:`  `
      (if (>= (`self.CompletedObjective`) (`KismetArrayLibrary.Array_Length` _activequest_questobjectives))
        (set `self.ActiveQuest` (struct))
        (set `self.CompletedObjective` 0)
        (`Widget.SetVisibility` (`/Game/BLUEPRINTS/UI/PlayerHUD.QuestComplete_WB` (`/Game/BLUEPRINTS/731Character.PlayerHUDref` (`self.As 731Character`))) "Visible")
        (`KismetSystemLibrary.Delay` 2.0)
        (`Widget.SetVisibility` (`/Game/BLUEPRINTS/UI/PlayerHUD.QuestComplete_WB` (`/Game/BLUEPRINTS/731Character.PlayerHUDref` (`self.As 731Character`))) "Hidden")
        (`Widget.SetVisibility` (`/Game/BLUEPRINTS/UI/PlayerHUD.ActiveQuest_WB` (`/Game/BLUEPRINTS/731Character.PlayerHUDref` (`self.As 731Character`))) "Hidden")
        (`Widget.SetVisibility` (`/Game/BLUEPRINTS/UI/PlayerHUD.ObjectiveBox` (`/Game/BLUEPRINTS/731Character.PlayerHUDref` (`self.As 731Character`))) "Hidden")
        (set `self.QuestCompleted?` true)))))