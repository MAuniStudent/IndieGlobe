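; Quest portal actor that saves the player's progress and opens a quest level when the 731Character walks into it.
; Tick spins the Quest mesh, while sphere overlap passes the character's save data to the game instance, waits briefly, destroys the actor and calls open level.
; The unlock visuals (green base with visible icon, or red base) are disconnected, and IsQuestUnlocked is never called, so entry is not gated.
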(event `self.ReceiveTick`
  (params (DeltaSeconds :type "Float (single-precision)"))
  (`SceneComponent.K2_AddRelativeRotation` (`self.Quest`) (struct :`Yaw` 1.0) false false))

(event `self.ReceiveBeginPlay`)

(event `self.Sphere.OnComponentBeginOverlap`
  (params (OverlappedComponent :type "PrimitiveComponent Object Reference") (OtherActor :type "Actor Object Reference") (OtherComp :type "PrimitiveComponent Object Reference") (OtherBodyIndex :type Integer) (bFromSweep :type Boolean) (SweepResult :type "HitResult Structure (by ref)"))
  (bind _as731character (cast `/Game/BLUEPRINTS/731Character` OtherActor))
  (bind _playerstats (`/Game/BLUEPRINTS/731Character.GetCurrentPlayerSaveData` _as731character))
  (message `/Game/BLUEPRINTS/savegame/BPI_SaveGame.SavePlayer` (`GameplayStatics.GetGameInstance`) _playerstats false)
  (`KismetSystemLibrary.Delay` 1.5)
  (`self.K2_DestroyActor`)
  (`GameplayStatics.OpenLevel` (`self.QuestToOpen`)))

(fn `IsQuestUnlocked`
  (returns (ReturnValue :type Boolean))
  (bind _playerstats (`/Game/BLUEPRINTS/731Character.GetCurrentPlayerSaveData` (`self.As 731Character`)))
  (return (>= (`.HighestQuestUnlocked_16_C457FA824C6C81C27ED51A95B13559F9` (break `/Game/BLUEPRINTS/savegame/PlayerStats_S` _playerstats)) (`self.PortalNumber`))))

(fn `UserConstructionScript`)