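; Game instance that owns the game's save data, loading it from a slot on Init or creating a new save object if none exists.
; Load and save events offer sync or async paths, with only a completed async load firing the OnGameLoad dispatcher.
; SavePlayer writes player stats into the cached save object before saving, and GetGameData exposes that object.
; Separate events show and hide a save prompt widget.
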(event `self.ReceiveInit`
  ;[1 1 1] Current game save loads when game starts
  (`self.LoadGameData` false))

(event `/Game/BLUEPRINTS/savegame/BPI_SaveGame.LoadGameData`
  (params (Async :type Boolean))
  ;[1 1 1] LOAD GAME
  (bind _returnvalue (`GameplayStatics.DoesSaveGameExist` (`self.SaveSlotName`)))
  (if _returnvalue
    (if Async
      ;;[0 0.1921 1 0.395] Loads game in background
      (bind _savegame (`AsyncActionHandleSaveGame.AsyncLoadGameFromSlot` (`self.SaveSlotName`))
        (:`Completed`
          (bind _as731save_game_bp (cast `/Game/BLUEPRINTS/savegame/731saveGame_BP` _savegame))
          (set `self.SavedGameData` _as731save_game_bp)
          (`self.OnGameLoad`)))
      (else
        ;;[0 0.1921 1 0.395] Loads game instantaniously
        (bind _returnvalue_2 (`GameplayStatics.LoadGameFromSlot` (`self.SaveSlotName`)))
        (bind _as731save_game_bp_2 (cast `/Game/BLUEPRINTS/savegame/731saveGame_BP` _returnvalue_2))
        (set `self.SavedGameData` _as731save_game_bp_2)))
    (else
      ;;[0 0.1921 1 0.395] If save game slot does not exist create one
      (bind _returnvalue_3 (`GameplayStatics.CreateSaveGameObject` "/Game/BLUEPRINTS/savegame/731saveGame_BP.731saveGame_BP_C"))
      (set `self.SavedGameData` _returnvalue_3))))

(event `ShowSavePrompt`
  ;[1 1 1] Save prompt in the backgroundfor Async save
  (bind _savewidgetref (`self.SaveWidgetREF`)
    (:`then`
      (`Widget.SetVisibility` _savewidgetref "Visible"))
    (:`else`
      (bind _returnvalue (`|CreateWidget` "/Game/BLUEPRINTS/UI/SavePrompt_WB.SavePrompt_WB_C"))
      (`UserWidget.AddToViewport` _returnvalue 0))))

(event `/Game/BLUEPRINTS/savegame/BPI_SaveGame.SaveGameData`
  (params (Async :type Boolean))
  ;[1 1 1] SAVE GAME
  (if Async
    (`AsyncActionHandleSaveGame.AsyncSaveGameToSlot` (`self.SavedGameData`) (`self.SaveSlotName`))
    (else
      (`GameplayStatics.SaveGameToSlot` (`self.SavedGameData`) (`self.SaveSlotName`)))))

(event `HideSavePrompt`
  ;[1 1 1] Save prompt in the backgroundfor Async save
  (bind _savewidgetref (`self.SaveWidgetREF`)
    (:`then`
      (`Widget.SetVisibility` _savewidgetref "Hidden"))
    (:`else`)))

(event `/Game/BLUEPRINTS/savegame/BPI_SaveGame.SavePlayer`
  (params (PlayerStats :type "/Game/BLUEPRINTS/savegame/PlayerStats_S Structure") (Async :type Boolean))
  ;[1 1 1] Save the current player stats, health, pickup count etc...
  (set `/Game/BLUEPRINTS/savegame/731saveGame_BP.PlayerSave` PlayerStats (`self.SavedGameData`))
  (`/Game/BLUEPRINTS/savegame/BPI_SaveGame.SaveGameData` Async))

(fn `GetGameData`
  (returns (SaveData :type "/Game/BLUEPRINTS/savegame/731saveGame_BP Object Reference"))
  (return (`self.SavedGameData`)))