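; Checkpoint actor that saves the player's stats when the 731Character overlaps its sphere.
; On overlap it gets the current player save from the character and passes it to the game instance's SavePlayerMessage with async off.
; It then plays a sound and shows a newly created save prompt widget, hiding it after a short delay without removing it.
; Nothing disables the trigger after a save.
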(event `self.Sphere.OnComponentBeginOverlap`
  (params (OverlappedComponent :type "PrimitiveComponent Object Reference") (OtherActor :type "Actor Object Reference") (OtherComp :type "PrimitiveComponent Object Reference") (OtherBodyIndex :type Integer) (bFromSweep :type Boolean) (SweepResult :type "HitResult Structure (by ref)"))
  (bind _as731character (cast `/Game/BLUEPRINTS/731Character` OtherActor))
  (set `self.As 731Character` _as731character)
  (bind _playerstats (`/Game/BLUEPRINTS/731Character.GetCurrentPlayerSave` (`self.As 731Character`)))
  (message `/Game/BLUEPRINTS/savegame/BPI_SaveGame.SavePlayer` (`GameplayStatics.GetGameInstance`) _playerstats false)
  (`GameplayStatics.PlaySound2D` "/Engine/EditorSounds/Notifications/CompileStart_Cue.CompileStart_Cue" 1.0 1.0 0.0 null null)
  (bind _returnvalue (`|CreateWidget` "/Game/BLUEPRINTS/UI/SavePrompt_WB.SavePrompt_WB_C"))
  (`UserWidget.AddToViewport` _returnvalue 0)
  (`Widget.SetVisibility` _returnvalue "Visible")
  (`KismetSystemLibrary.Delay` 1.5)
  (`Widget.SetVisibility` _returnvalue "Hidden")
  (`KismetSystemLibrary.PrintString` "Player Stats Saved"))

(fn `UserConstructionScript`)