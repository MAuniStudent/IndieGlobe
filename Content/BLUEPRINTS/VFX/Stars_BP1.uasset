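; Collectible star pickup that the player character gathers by overlapping its sphere.
; On overlap it increments the character's Stars count, plays a ping and spawns a small-star Niagara effect at its location.
; The effect spawns inactive, gets its "User.place" variable set from the player's X and raised Z, then activates.
; The star then destroys itself and reports to the character's quest component for collection objectives.
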(event `self.Sphere.OnComponentBeginOverlap`
  (params (OverlappedComponent :type "PrimitiveComponent Object Reference") (OtherActor :type "Actor Object Reference") (OtherComp :type "PrimitiveComponent Object Reference") (OtherBodyIndex :type Integer) (bFromSweep :type Boolean) (SweepResult :type "HitResult Structure (by ref)"))
  ;[0 0.1921 1 0.395] On Player Overlap Plus 1 to star count
  (bind _as731character (cast `/Game/BLUEPRINTS/731Character` OtherActor))
  (bind _output_get (set `self.As BP Third Person Character` _as731character))
  (set `/Game/BLUEPRINTS/731Character.Stars` (+ (`/Game/BLUEPRINTS/731Character.Stars` _output_get) 1) _output_get)
  (`GameplayStatics.PlaySound2D` "/Engine/EngineSounds/1kSineTonePing.1kSineTonePing" 1.0 1.0 0.0 null null)
  (bind _returnvalue (`NiagaraFunctionLibrary.SpawnSystemAtLocation` "/Game/BLUEPRINTS/VFX/System/NS_StarSmall.NS_StarSmall" (`self.K2_GetActorLocation` self) (struct) (1.0 1.0 1.0) true false))
  (`NiagaraComponent.SetVariablePosition` _returnvalue "User.place" (`KismetMathLibrary.MakeVector` (.x (`self.K2_GetActorLocation` _as731character)) 0.0 (+ (.z (`self.K2_GetActorLocation` _as731character)) 100.0)))
  (`ActorComponent.Activate` _returnvalue false)
  (`self.K2_DestroyActor`)
  ;;[0 1 0.6156] Targeted at quest objectives for each STAR collected
  (`/Game/BLUEPRINTS/savegame/QuestSystem/BPC_Quests.CollectOrEndActors` (`/Game/BLUEPRINTS/731Character.BPC_Quests` (`self.As BP Third Person Character`)) self))

(fn `UserConstructionScript`)