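; Interactable computer chair that seats the 731 character at a PC and switches play to on-screen use.
; Interact toggles movement, slides the character onto the seat with sit and type montages, blends the view to the chair, hides the HUD and focuses the screen widget with a cursor.
; After a delay it pings and enables its own input.
; DontInteract moves the character to the Standing point and restores view, HUD and game input.
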(event `self.ReceiveBeginPlay`
  (`parent.ReceiveBeginPlay`))

(event `self.Interact`
  (bind _returnvalue (`GameplayStatics.GetPlayerController` 0))
  (bind (_returnvalue_roll _returnvalue_pitch _returnvalue_yaw) (`KismetMathLibrary.BreakRotator` (`self.K2_GetActorRotation`)))
  (bind _as_731character (`self.As 731Character`))
  (`parent.Interact`)
  (bind _as731character (cast `/Game/BLUEPRINTS/731Character` (`self.DelegateActor`)))
  (bind _output_get (set `self.As 731Character` _as731character))
  ;[1 1 1] toggle control movement
  (message `/Game/BLUEPRINTS/Interactables/WorldInteractableObjects/ObjectInteraction_BPI.ToggleMovement` _output_get false)
  (`Character.PlayAnimMontage` (`self.As 731Character`) "/Game/Characters/Mixamo/MixamoAnimations/ue5/Sitting_Montage.Sitting_Montage" 1.0 "None")
  (`KismetSystemLibrary.MoveComponentTo` (`Actor.RootComponent` _as_731character) (+ (`self.K2_GetActorLocation`) (`KismetMathLibrary.MakeVector` 0.0 0.0 (`CapsuleComponent.CapsuleHalfHeight` (`Character.CapsuleComponent` _as_731character)))) (`KismetMathLibrary.MakeRotator` 0.0 0.0 (+ _returnvalue_yaw 90.0)) false false 1.0)
  (`PlayerController.SetViewTargetWithBlend` (`GameplayStatics.GetPlayerController` 0) self 2.0 "VTBlend_Linear" 0.0 true)
  (`Character.PlayAnimMontage` (`self.As 731Character`) "/Game/Characters/Mixamo/MixamoAnimations/ue5/Typing_Montage.Typing_Montage" 1.0 "None")
  (`WidgetBlueprintLibrary.SetInputMode_GameAndUIEx` _returnvalue (`self.ScreenREF`))
  (set `PlayerController.bShowMouseCursor` true _returnvalue)
  (set `self.IsUsingPC?` true)
  (`Widget.SetVisibility` (`/Game/BLUEPRINTS/731Character.PlayerHUDref` (`self.As 731Character`)) "Hidden")
  (`KismetSystemLibrary.Delay` 4.0)
  (`GameplayStatics.PlaySound2D` "/Engine/EngineSounds/1kSineTonePing.1kSineTonePing" 1.0 1.0 0.0 null null)
  (`self.EnableInput` self _returnvalue))

(event `self.DontInteract`
  (bind _returnvalue (`GameplayStatics.GetPlayerController` 0))
  (bind _as_731character (`self.As 731Character`))
  (`parent.DontInteract`)
  (bind _as_731character_2 (`self.As 731Character`)
    (:`then`
      (`Character.StopAnimMontage` _as_731character_2 null)
      (`WidgetBlueprintLibrary.SetInputMode_GameOnly` _returnvalue)
      (set `PlayerController.bShowMouseCursor` false _returnvalue)
      (`Character.PlayAnimMontage` (`self.As 731Character`) "/Game/Characters/Mixamo/MixamoAnimations/ue5/Sit_To_Stand_Montage.Sit_To_Stand_Montage" 1.0 "None")
      (`KismetSystemLibrary.MoveComponentTo` (`Actor.RootComponent` _as_731character) (+ (`KismetMathLibrary.MakeVector` 0.0 0.0 (`CapsuleComponent.CapsuleHalfHeight` (`Character.CapsuleComponent` _as_731character))) (`SceneComponent.K2_GetComponentLocation` (`self.Standing`))) (`self.K2_GetActorRotation`) false false 0.5)
      (message `/Game/BLUEPRINTS/Interactables/WorldInteractableObjects/ObjectInteraction_BPI.ToggleMovement` _as_731character_2 true)
      (set `self.IsUsingPC?` false)
      (`PlayerController.SetViewTargetWithBlend` (`GameplayStatics.GetPlayerController` 0) (`self.As 731Character`) 2.0 "VTBlend_Linear" 0.0 false)
      (`Widget.SetVisibility` (`/Game/BLUEPRINTS/731Character.PlayerHUDref` (`self.As 731Character`)) "Visible"))
    (:`else`)))

(fn `UserConstructionScript`
  (`parent.UserConstructionScript`))