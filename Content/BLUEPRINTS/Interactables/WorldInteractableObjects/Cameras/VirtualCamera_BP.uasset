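; Virtual camera actor that captures the scene and feeds the image to linked screen actors.
; Shortly after BeginPlay, it creates a canvas render target for its SceneCapture2D and passes the texture to each ScreenREF entry through CameraTextureMessage.
; A CameraRotation event uses a timeline to turn the camera anchor in repeating 25-degree steps with pauses between them, but its starting call in this graph is disconnected.
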(event `self.ReceiveBeginPlay`
  (`KismetSystemLibrary.Delay` 0.2)
  ;[1 1 1] Setup scene capture component for virtual camera
  (bind _returnvalue (`CanvasRenderTarget2D.CreateCanvasRenderTarget2D` "/Script/Engine.CanvasRenderTarget2D"))
  (bind _output_get (set `SceneCaptureComponent2D.TextureTarget` _returnvalue (`self.SceneCaptureComponent2D`)))
  (for _array_element (`self.ScreenREF`)
    (message `/Game/BLUEPRINTS/Interactables/WorldInteractableObjects/Cameras/BPI_VirtualCameraControls.CameraTexture` _array_element _output_get)))

(event `CameraRotation`
  ;[1 1 1] Setup rotation for camera
  (bind _output_get (set `self.StartRotation` (`SceneComponent.K2_GetComponentRotation` (`self.CameraAnchor`))))
  (set `self.TargetRotation` (`KismetMathLibrary.ComposeRotators` _output_get (struct :`Yaw` 25.0)))
  (bind (_direction _rotation) (`Timeline|CameraRotator` :!via `PlayFromStart`)
    (:`Update`
      (`SceneComponent.K2_SetWorldRotation` (`self.CameraAnchor`) (`KismetMathLibrary.RLerp` (`self.StartRotation`) (`self.TargetRotation`) _rotation true) false false))
    (:`Finished`
      (`KismetSystemLibrary.Delay` 1.0)
      (`self.CameraRotation`))))

(fn `UserConstructionScript`)