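; ActiveComputer_BP is an interactable world computer that switches its display on while the player character is nearby.
; When a 731Character enters its Sphere, it shows the UserInterface component and applies the monitor display material to the Screen's second material slot.
; When the character leaves, it hides the interface and swaps in M_Cooking_surface, apparently as the screen-off look.
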(event `self.ReceiveBeginPlay`)

(event `self.Sphere.OnComponentBeginOverlap`
  (params (OverlappedComponent :type "PrimitiveComponent Object Reference") (OtherActor :type "Actor Object Reference") (OtherComp :type "PrimitiveComponent Object Reference") (OtherBodyIndex :type Integer) (bFromSweep :type Boolean) (SweepResult :type "HitResult Structure (by ref)"))
  (cast `/Game/BLUEPRINTS/731Character` OtherActor)
  (`SceneComponent.SetVisibility` (`self.UserInterface`) true false)
  (`PrimitiveComponent.SetMaterial` (`self.Screen`) 1 "/Game/TP_Assets/LoftOffice/Materials/M_Monitor_display.M_Monitor_display"))

(event `self.Sphere.OnComponentEndOverlap`
  (params (OverlappedComponent :type "PrimitiveComponent Object Reference") (OtherActor :type "Actor Object Reference") (OtherComp :type "PrimitiveComponent Object Reference") (OtherBodyIndex :type Integer))
  (cast `/Game/BLUEPRINTS/731Character` OtherActor)
  (`SceneComponent.SetVisibility` (`self.UserInterface`) false false)
  (`PrimitiveComponent.SetMaterial` (`self.Screen`) 1 "/Game/TP_Assets/LoftOffice/Materials/M_Cooking_surface.M_Cooking_surface"))

(fn `UserConstructionScript`)