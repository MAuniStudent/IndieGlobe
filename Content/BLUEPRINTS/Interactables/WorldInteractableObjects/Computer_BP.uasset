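; Computer interactable that shows or hides its ComputerScreen based on whether its owning ComputerChair_BP is in use.
; On BeginPlay it casts its owner to the chair and reads IsUsingPC once, with no later updates.
; If true, it reveals the screen, switches the first player to UI-only input with a mouse cursor and prints a debug message.
; Otherwise it hides the screen.
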(event `self.ReceiveBeginPlay`
  (bind _returnvalue (`GameplayStatics.GetPlayerController` 0))
  (bind _ascomputer_chair_bp (cast `/Game/BLUEPRINTS/Interactables/WorldInteractableObjects/ComputerChair_BP` (`self.GetOwner`)))
  (if (`/Game/BLUEPRINTS/Interactables/WorldInteractableObjects/ComputerChair_BP.IsUsingPC?` _ascomputer_chair_bp)
    (`SceneComponent.SetHiddenInGame` (`self.ComputerScreen`) false false)
    (`WidgetBlueprintLibrary.SetInputMode_UIOnlyEx` _returnvalue null)
    (set `PlayerController.bShowMouseCursor` true _returnvalue)
    (`KismetSystemLibrary.PrintString` "IS USING PC")
    (else
      (`SceneComponent.SetHiddenInGame` (`self.ComputerScreen`) true false))))

(fn `UserConstructionScript`)