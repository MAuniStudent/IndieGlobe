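; Interactable world object that shows a prompt and accepts the interaction input while the player character is inside its box trigger.
; Overlap events identify the player through a PlayerCharacterMessage call, store it as DelegateActor on entry, and toggle the prompt and actor input.
; IA_Interaction alternates between Interact and DontInteract events, which only flip IsInteracting and hide or reshow the prompt.
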(event `self.Box.OnComponentBeginOverlap`
  (params (OverlappedComponent :type "PrimitiveComponent Object Reference") (OtherActor :type "Actor Object Reference") (OtherComp :type "PrimitiveComponent Object Reference") (OtherBodyIndex :type Integer) (bFromSweep :type Boolean) (SweepResult :type "HitResult Structure (by ref)"))
  (bind _active (message `/Game/BLUEPRINTS/Interactables/WorldInteractableObjects/ObjectInteraction_BPI.PlayerCharacter?` OtherActor))
  (if _active
    (set `self.DelegateActor` OtherActor)
    (`SceneComponent.SetVisibility` (`self.InteractionPrompt`) true false)
    (`self.EnableInput` (`GameplayStatics.GetPlayerController` 0))))

(event `self.Box.OnComponentEndOverlap`
  (params (OverlappedComponent :type "PrimitiveComponent Object Reference") (OtherActor :type "Actor Object Reference") (OtherComp :type "PrimitiveComponent Object Reference") (OtherBodyIndex :type Integer))
  (bind _active (message `/Game/BLUEPRINTS/Interactables/WorldInteractableObjects/ObjectInteraction_BPI.PlayerCharacter?` OtherActor))
  (if _active
    (`SceneComponent.SetVisibility` (`self.InteractionPrompt`) false false)
    (`self.DisableInput` (`GameplayStatics.GetPlayerController` 0))))

(event `EnhancedInput|/Game/BLUEPRINTS/Input/Actions/IA_Interaction`
  (params (ActionValue :type Boolean) (ElapsedSeconds :type "Float (double-precision)") (TriggeredSeconds :type "Float (double-precision)") (InputAction :type "InputAction Object Reference" :default "/Game/BLUEPRINTS/Input/Actions/IA_Interaction.IA_Interaction"))
  (:`Started`
    (if (`self.IsInteracting?`)
      (`self.DontInteract`)
      (else
        (`self.Interact`)))))

(event `Interact`
  (set `self.IsInteracting?` true)
  (`SceneComponent.SetVisibility` (`self.InteractionPrompt`) false false))

(event `DontInteract`
  (set `self.IsInteracting?` false)
  (`SceneComponent.SetVisibility` (`self.InteractionPrompt`) true false))

(fn `UserConstructionScript`)