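; HiFi_BP is an interactable hi-fi radio that can play a music track at its location.
; A sphere overlap with the player character shows the Interaction widget with a turn on/off prompt and sets CanPlayMusic; leaving only hides the widget.
; The track plays only if that flag is already true at BeginPlay.
; No input handling or stop logic exists here, so the prompt's toggle is not implemented in this graph.
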(event `self.ReceiveBeginPlay`
  (if (`self.CanPlayMusic?`)
    (`GameplayStatics.PlaySoundAtLocation` "/Game/BLUEPRINTS/Music/IGD_SectorFour.IGD_SectorFour" (`self.K2_GetActorLocation` self) (struct) 1.0 1.0 0.0 null null null null)))

(event `self.Sphere.OnComponentBeginOverlap`
  (params (OverlappedComponent :type "PrimitiveComponent Object Reference") (OtherActor :type "Actor Object Reference") (OtherComp :type "PrimitiveComponent Object Reference") (OtherBodyIndex :type Integer) (bFromSweep :type Boolean) (SweepResult :type "HitResult Structure (by ref)"))
  (bind _as731character (cast `/Game/BLUEPRINTS/731Character` OtherActor))
  (set `self.As 731Character` _as731character)
  (`SceneComponent.SetVisibility` (`self.Interaction`) true false)
  (bind _asuse_prompt_wb (cast `/Game/BLUEPRINTS/UI/UsePrompt_WB` (`WidgetComponent.GetUserWidgetObject` (`self.Interaction`))))
  (`TextBlock.SetText` (`/Game/BLUEPRINTS/UI/UsePrompt_WB.UseText` _asuse_prompt_wb) "Turn On/Off [ E ]")
  (set `self.CanPlayMusic?` true))

(event `self.Sphere.OnComponentEndOverlap`
  (params (OverlappedComponent :type "PrimitiveComponent Object Reference") (OtherActor :type "Actor Object Reference") (OtherComp :type "PrimitiveComponent Object Reference") (OtherBodyIndex :type Integer))
  (bind _as731character (cast `/Game/BLUEPRINTS/731Character` OtherActor))
  (set `self.As 731Character` _as731character)
  (`SceneComponent.SetVisibility` (`self.Interaction`) false false))

(fn `UserConstructionScript`)