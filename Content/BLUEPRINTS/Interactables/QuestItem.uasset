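; QuestItem is an interactable pickup that the player character collects by walking into its sphere trigger.
; On overlap with 731Character, it increments the character's Key count, sets the HUD pickup icon and reveals the quest item widget.
; It then plays a ping sound, destroys itself and afterwards passes itself to the character's BPCQuests component through CollectOrEndActors.
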(event `self.Sphere.OnComponentBeginOverlap`
  (params (OverlappedComponent :type "PrimitiveComponent Object Reference") (OtherActor :type "Actor Object Reference") (OtherComp :type "PrimitiveComponent Object Reference") (OtherBodyIndex :type Integer) (bFromSweep :type Boolean) (SweepResult :type "HitResult Structure (by ref)"))
  (bind _as731character (cast `/Game/BLUEPRINTS/731Character` OtherActor))
  (bind _output_get (set `self.As BP Third Person Character` _as731character))
  (set `/Game/BLUEPRINTS/731Character.Key` (+ (`/Game/BLUEPRINTS/731Character.Key` _output_get) 1) _output_get)
  (bind _playerhudref (`/Game/BLUEPRINTS/731Character.PlayerHUDref` _output_get))
  (set `/Game/BLUEPRINTS/UI/PlayerHUD.PickupIcon` (`self.QuestItemIcon`) _playerhudref)
  (`Widget.SetVisibility` (`/Game/BLUEPRINTS/UI/PlayerHUD.QuestItem` _playerhudref) "Visible")
  (`GameplayStatics.PlaySound2D` "/Engine/EngineSounds/1kSineTonePing.1kSineTonePing" 1.0 1.0 0.0 null null)
  (`self.K2_DestroyActor`)
  ;[1 1 1] Collect or destroy the object
  (`/Game/BLUEPRINTS/savegame/QuestSystem/BPC_Quests.CollectOrEndActors` (`/Game/BLUEPRINTS/731Character.BPC_Quests` (`self.As BP Third Person Character`)) self))

(fn `UserConstructionScript`)