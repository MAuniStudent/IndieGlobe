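; Reward chest actor that opens to reveal a spinning star and return a reward item.
; At BeginPlay it toggles its root's visibility from the character's quest-completed flag, through a reference otherwise assigned only on overlap or opening.
; Sphere overlap shows or hides the interaction prompt.
; OpenChest plays the animation, unhides both star components, notifies the player's BPCQuests component and returns RewardedItem.
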(event `self.ReceiveBeginPlay`
  (if (`/Game/BLUEPRINTS/savegame/QuestSystem/BPC_Quests.QuestCompleted?` (`/Game/BLUEPRINTS/731Character.BPC_Quests` (`self.As 731Character`)))
    (`SceneComponent.SetHiddenInGame` (`self.DefaultSceneRoot`) false false)
    (else
      (`SceneComponent.SetHiddenInGame` (`self.DefaultSceneRoot`) true false))))

(event `self.ReceiveTick`
  (params (DeltaSeconds :type "Float (single-precision)"))
  (`SceneComponent.K2_AddRelativeRotation` (`self.Star`) (struct :`Yaw` 3.0) false false))

(event `self.Sphere.OnComponentBeginOverlap`
  (params (OverlappedComponent :type "PrimitiveComponent Object Reference") (OtherActor :type "Actor Object Reference") (OtherComp :type "PrimitiveComponent Object Reference") (OtherBodyIndex :type Integer) (bFromSweep :type Boolean) (SweepResult :type "HitResult Structure (by ref)"))
  (bind _as731character (cast `/Game/BLUEPRINTS/731Character` OtherActor))
  (set `self.As 731Character` _as731character)
  (`SceneComponent.SetVisibility` (`self.InteractionPrompt`) true false))

(event `self.Sphere.OnComponentEndOverlap`
  (params (OverlappedComponent :type "PrimitiveComponent Object Reference") (OtherActor :type "Actor Object Reference") (OtherComp :type "PrimitiveComponent Object Reference") (OtherBodyIndex :type Integer))
  (bind _as731character (cast `/Game/BLUEPRINTS/731Character` OtherActor))
  (set `self.As 731Character` _as731character)
  (`SceneComponent.SetVisibility` (`self.InteractionPrompt`) false false))

(fn `OpenChest`
  (returns (Item :type "/Game/BLUEPRINTS/Interactables/ChestReward/ChestRewards_S Structure"))
  (bind _as731character (cast `/Game/BLUEPRINTS/731Character` (`GameplayStatics.GetPlayerCharacter` 0)))
  (`SkeletalMeshComponent.PlayAnimation` (`self.Chest`) "/Game/BLUEPRINTS/Meshs/SkeletalMesh/Chest_Open.Chest_Open" false)
  (`SceneComponent.SetHiddenInGame` (`self.Star`) false false)
  (`SceneComponent.SetHiddenInGame` (`self.InnerStar`) false false)
  (`/Game/BLUEPRINTS/savegame/QuestSystem/BPC_Quests.OpenRewardChest` (`/Game/BLUEPRINTS/731Character.BPC_Quests` _as731character) self)
  (return (`self.RewardedItem`)))

(fn `UserConstructionScript`)