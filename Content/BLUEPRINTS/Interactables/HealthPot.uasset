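; HealthPot is a health pickup that heals the player character (731Character) when it overlaps the pot's sphere.
; The overlap adds a fixed amount to Health, then sets it to MaxHealth if it reaches a hardcoded 100 threshold, rather than comparing against MaxHealth.
; It plays a 2D sound, destroys itself and prints on-screen messages for the heal and for full health.
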(event `self.Sphere.OnComponentBeginOverlap`
  (params (OverlappedComponent :type "PrimitiveComponent Object Reference") (OtherActor :type "Actor Object Reference") (OtherComp :type "PrimitiveComponent Object Reference") (OtherBodyIndex :type Integer) (bFromSweep :type Boolean) (SweepResult :type "HitResult Structure (by ref)"))
  (bind _as731character (cast `/Game/BLUEPRINTS/731Character` OtherActor))
  (bind _output_get (set `/Game/BLUEPRINTS/731Character.Health` (+ (`/Game/BLUEPRINTS/731Character.Health` _as731character) 25.0) _as731character))
  (if (>= _output_get 100.0)
    (set `/Game/BLUEPRINTS/731Character.Health` (`/Game/BLUEPRINTS/731Character.MaxHealth` _as731character) _as731character)
    (`KismetSystemLibrary.PrintString` "Health Is Full!" true true (struct :`R` 1.0 :`G` 0.03877 :`A` 1.0)))
  (`GameplayStatics.PlaySound2D` "/Engine/VREditor/Sounds/UI/Camera_Shutter.Camera_Shutter" 1.0 1.0 0.0 null null)
  (`self.K2_DestroyActor`)
  (`KismetSystemLibrary.PrintString` "Health increased by 25" true true (struct :`R` 1.0 :`B` 0.04262 :`A` 1.0)))

(fn `UserConstructionScript`)