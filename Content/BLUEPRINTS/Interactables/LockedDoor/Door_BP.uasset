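; Locked door actor that the 731Character can open and close once they hold at least one key.
; Box overlap turns on the door's custom depth and a widget, which shows either an open prompt or a find-key message.
; Enhanced Input interaction, gated by CanOpen, toggles between two timelines that offset the actor's yaw from its BeginPlay rotation, with CloseDoor played in reverse.
; The key count is only checked, never decremented.
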(event `self.ReceiveBeginPlay`
  (set `self.CurrentDoor_Z_Rotation` (`self.K2_GetActorRotation`)))

(event `self.Box.OnComponentBeginOverlap`
  (params (OverlappedComponent :type "PrimitiveComponent Object Reference") (OtherActor :type "Actor Object Reference") (OtherComp :type "PrimitiveComponent Object Reference") (OtherBodyIndex :type Integer) (bFromSweep :type Boolean) (SweepResult :type "HitResult Structure (by ref)"))
  (bind _as731character (cast `/Game/BLUEPRINTS/731Character` OtherActor))
  (set `self.As 731Character` _as731character)
  (`PrimitiveComponent.SetRenderCustomDepth` (`self.Door`) true)
  (`SceneComponent.SetVisibility` (`self.Widget`) true false)
  (if (>= (`/Game/BLUEPRINTS/731Character.Key` (`self.As 731Character`)) 1)
    (bind _asopen_door_wb (cast `/Game/BLUEPRINTS/UI/OpenDoor_WB` (`WidgetComponent.GetUserWidgetObject` (`self.Widget`))))
    (set `/Game/BLUEPRINTS/UI/OpenDoor_WB.KeyInfo` "Open [ E ]" _asopen_door_wb)
    (`self.EnableInput` (`GameplayStatics.GetPlayerController` 0))
    (set `self.CanOpen?` true)
    (else
      (bind _asopen_door_wb_2 (cast `/Game/BLUEPRINTS/UI/OpenDoor_WB` (`WidgetComponent.GetUserWidgetObject` (`self.Widget`))))
      (set `/Game/BLUEPRINTS/UI/OpenDoor_WB.KeyInfo` "Find the door key!" _asopen_door_wb_2)
      (set `self.CanOpen?` false))))

(event `self.Box.OnComponentEndOverlap`
  (params (OverlappedComponent :type "PrimitiveComponent Object Reference") (OtherActor :type "Actor Object Reference") (OtherComp :type "PrimitiveComponent Object Reference") (OtherBodyIndex :type Integer))
  (bind _as731character (cast `/Game/BLUEPRINTS/731Character` OtherActor))
  (set `self.As 731Character` _as731character)
  (`PrimitiveComponent.SetRenderCustomDepth` (`self.Door`) false)
  (`SceneComponent.SetVisibility` (`self.Widget`) false false)
  (set `self.CanOpen?` false))

(event `EnhancedInput|/Game/BLUEPRINTS/Input/Actions/IA_Interaction`
  (params (ActionValue :type Boolean) (ElapsedSeconds :type "Float (double-precision)") (TriggeredSeconds :type "Float (double-precision)") (InputAction :type "InputAction Object Reference" :default "/Game/BLUEPRINTS/Input/Actions/IA_Interaction.IA_Interaction"))
  (bind (_currentdoor_z_rotation_roll _currentdoor_z_rotation_pitch _currentdoor_z_rotation_yaw) (`KismetMathLibrary.BreakRotator` (`self.CurrentDoor_Z_Rotation`)))
  (bind (_currentdoor_z_rotation_roll_2 _currentdoor_z_rotation_pitch_2 _currentdoor_z_rotation_yaw_2) (`KismetMathLibrary.BreakRotator` (`self.CurrentDoor_Z_Rotation`)))
  (:`Started`
    (if (`self.CanOpen?`)
      (if (`self.IsDoorOpen?`)
        (bind (_direction _open) (`Timeline|CloseDoor` :!via `ReverseFromEnd`)
          (:`Update`
            (`self.K2_SetActorRelativeRotation` (`KismetMathLibrary.MakeRotator` 0.0 0.0 (+ _currentdoor_z_rotation_yaw _open)))
            (set `self.IsDoorOpen?` false)
            (`KismetSystemLibrary.PrintString` "Close Door")))
        (else
          (bind (_direction_2 _open_2) (`Timeline|OpenDoor` :!via `PlayFromStart`)
            (:`Update`
              (`self.K2_SetActorRelativeRotation` (`KismetMathLibrary.MakeRotator` 0.0 0.0 (+ _currentdoor_z_rotation_yaw_2 _open_2)))
              (set `self.IsDoorOpen?` true)
              (`KismetSystemLibrary.PrintString` "Open Door"))))))))

(fn `UserConstructionScript`)