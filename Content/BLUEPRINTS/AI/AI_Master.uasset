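; AI_Master is an AI character Blueprint that wanders randomly and displays its name on a widget.
; On BeginPlay it sets the name text and starting health, and a looping timer turns the widget toward the player camera.
; Movement picks random reachable points nearby and repeats after a delay, only when a move succeeds.
; The construction script makes the modular body meshes follow the main Mesh's pose.
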(event `Start`
  ;[1 1 1] Name widget faces player position
  (`KismetSystemLibrary.K2_SetTimerDelegate` (delegate `TurnWidget`) 0.2 true))

(event `TurnWidget`
  (bind _name (`self.Name`))
  ;[1 1 1] Name widget faces player position
  (`SceneComponent.K2_SetWorldRotation` _name (`KismetMathLibrary.FindLookAtRotation` (`SceneComponent.K2_GetComponentLocation` _name) (`PlayerCameraManager.GetCameraLocation` (`GameplayStatics.GetPlayerCameraManager` 0))) false false))

(event `self.ReceiveBeginPlay`
  (`self.Start`)
  (bind _asname_wb (cast `/Game/BLUEPRINTS/UI/Name_WB` (`WidgetComponent.GetUserWidgetObject` (`self.Name`))))
  (`TextBlock.SetText` (`/Game/BLUEPRINTS/UI/Name_WB.AI_name` _asname_wb) (`self.NameOfAI`))
  (set `self.Currenthealth` 100.0)
  (`self.RandomAI_Movement`))

(event `RandomAI_Movement`
  (`|AIMoveTo` self (`NavigationSystemV1.K2_GetRandomReachablePointInRadius` (`self.K2_GetActorLocation`) 2500.0 null "/Script/AIModule.NavFilter_AIControllerDefault") null
    (:`OnSuccess`
      (`KismetSystemLibrary.Delay` 4.0)
      (`self.RandomAI_Movement`))))

(fn `UserConstructionScript`
  (`SkinnedMeshComponent.SetLeaderPoseComponent` (`self.UpperBody`) (`self.Mesh`) true true)
  (`SkinnedMeshComponent.SetLeaderPoseComponent` (`self.Arms`) (`self.Mesh`) true true)
  (`SkinnedMeshComponent.SetLeaderPoseComponent` (`self.LowerBody`) (`self.Mesh`) true true)
  (`SkinnedMeshComponent.SetLeaderPoseComponent` (`self.Feet`) (`self.Mesh`) true true))