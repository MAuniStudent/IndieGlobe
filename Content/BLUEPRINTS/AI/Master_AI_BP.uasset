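; Master AI character Blueprint that provides a modular body and a displayed name for AI characters.
; The construction script sets the main Mesh as leader pose for the face prop, hair/hat, feet, hands, upper body and lower body, so the parts animate together.
; On BeginPlay, it casts the Name component's widget to Name_WB and writes NameOfCharacter into its AIName text.
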(event `self.ReceiveBeginPlay`
  ;[1 1 1] Set The Name of AI character
  (bind _asname_wb (cast `/Game/BLUEPRINTS/UI/Name_WB` (`WidgetComponent.GetUserWidgetObject` (`self.Name`))))
  (`TextBlock.SetText` (`/Game/BLUEPRINTS/UI/Name_WB.AI_name` _asname_wb) (`self.NameOfCharacter`)))

(fn `UserConstructionScript`
  (`SkinnedMeshComponent.SetLeaderPoseComponent` (`self.FaceProp`) (`self.Mesh`) false false)
  (`SkinnedMeshComponent.SetLeaderPoseComponent` (`self.Hair/Hat`) (`self.Mesh`) false false)
  (`SkinnedMeshComponent.SetLeaderPoseComponent` (`self.Feet`) (`self.Mesh`) false false)
  (`SkinnedMeshComponent.SetLeaderPoseComponent` (`self.Hands`) (`self.Mesh`) false false)
  (`SkinnedMeshComponent.SetLeaderPoseComponent` (`self.UpperBody`) (`self.Mesh`) false false)
  (`SkinnedMeshComponent.SetLeaderPoseComponent` (`self.LowerBody`) (`self.Mesh`) false false))