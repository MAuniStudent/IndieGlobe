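; Procedural wall Blueprint that builds a grid of mesh pieces from XValue columns and YValue rows.
; The construction script loops over both counts and adds an instance to an InstancedStaticMesh at each cell, in local space along X and Z.
; Spacing is hard-coded at 256 units to match the mesh size.
; The event graph is empty, so all work happens at construction.
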(fn `UserConstructionScript`
  (locals (LooopX_Value :type Integer) (LooopY_Value :type Integer))
  (for _index (range (`self.X_Value`))
    (set `local.LooopX_Value` _index)
    (for _index_2 (range (`self.Y_Value`))
      (set `local.LooopY_Value` _index_2)
      (`InstancedStaticMeshComponent.AddInstance` (`self.InstancedStaticMesh`) (`KismetMathLibrary.MakeTransform` (`KismetMathLibrary.MakeVector` (* (`local.LooopX_Value`) 256.0) 0.0 (* (`local.LooopY_Value`) 256.0))) false))))