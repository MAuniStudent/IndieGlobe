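; Master Blueprint for modular AI characters with a floating name widget, facial morph animation and a basic move to a random point.
; Construction script makes body, footwear and head prop meshes follow the main Mesh via leader pose.
; On BeginPlay, a timeline drives the Smile_01 morph (commented as a blink) and rewrites the name text on each update.
; A single AIMoveTo targets a random nearby reachable point, only printing a message on arrival.
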(event `self.ReceiveBeginPlay`
  ;[1 1 1] Morph Targets
  (`|ExecutionSequence`
    (:`then_0`
      (bind (_direction _newtrack_0) (`Timeline|Timeline_0`) ; Timeline length is 4, one blink every 4 seconds.
        (:`Update`
          (`SkeletalMeshComponent.SetMorphTarget` (`self.Mesh`) "Smile_01" _newtrack_0 true)
          (bind _asname_wb (cast `/Game/BLUEPRINTS/UI/Name_WB` (`WidgetComponent.GetUserWidgetObject` (`self.Name`))))
          (`TextBlock.SetText` (`/Game/BLUEPRINTS/UI/Name_WB.AI_name` _asname_wb) (`self.AI Name`)))))
    (:`then_1`
      (`|AIMoveTo` self (`NavigationSystemV1.K2_GetRandomReachablePointInRadius` (`self.K2_GetActorLocation`) 1000.0 null null) null
        (:`OnSuccess`
          (`KismetSystemLibrary.PrintString` "Now where do i go"))))))

(fn `UserConstructionScript`
  (`SkinnedMeshComponent.SetLeaderPoseComponent` (`self.Lower Body`) (`self.Mesh`) false false)
  (`SkinnedMeshComponent.SetLeaderPoseComponent` (`self.Footwear 01`) (`self.Mesh`) false false)
  (`SkinnedMeshComponent.SetLeaderPoseComponent` (`self.Upper Body`) (`self.Mesh`) false false)
  (`SkinnedMeshComponent.SetLeaderPoseComponent` (`self.Body Parts 01`) (`self.Mesh`) false false)
  (`SkinnedMeshComponent.SetLeaderPoseComponent` (`self.Footwear 02`) (`self.Mesh`) false false)
  (`SkinnedMeshComponent.SetLeaderPoseComponent` (`self.Props Head 01`) (`self.Mesh`) false false))