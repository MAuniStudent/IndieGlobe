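; Wave spawner for minigames that chains to the next spawner or shows the victory screen once all its spawned items are gone.
; SpawnObjects spawns each ItemsToSpawn marker's Item class at that marker's location and tracks it in Items, optionally on BeginPlay.
; While Active, Tick prunes invalid items; when none remain, it triggers and activates NextSpawner, or calls MiniGameCharacter's VictoryScreen, then destroys itself.
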(event `self.ReceiveBeginPlay`
  (if (`self.SpawnOnStart`)
    (`self.SpawnObjects`)))

(event `self.ReceiveTick`
  (params (DeltaSeconds :type "Float (single-precision)"))
  (bind _items (`self.Items`))
  (bind _nextspawner (`self.NextSpawner`))
  (if (`self.Active`)
    (`/Engine/EditorBlueprintResources/StandardMacros.DoOnce` false :!label _label
      (:`Completed`
        (for _array_element _items
          (if (not (`KismetSystemLibrary.IsValid` _array_element))
            (`KismetArrayLibrary.Array_RemoveItem` _items _array_element)
            (break)))
        (if (<= (`KismetArrayLibrary.Array_Length` _items) 0)
          (if (`KismetSystemLibrary.IsValid` _nextspawner)
            (`self.SpawnObjects` _nextspawner)
            (set `/Game/MiniGames/Blueprints/ObjectSpawner.Active` true _nextspawner)
            (else
              (bind _returnvalue (`GameplayStatics.GetActorOfClass` "/Game/MiniGames/Blueprints/MiniGameCharacter.MiniGameCharacter_C"))
              (`/Game/MiniGames/Blueprints/MiniGameCharacter.Victory Screen` _returnvalue)))
          (`self.K2_DestroyActor`)
          (else
            (goto _label :!via `Reset`)))))))

(fn `SpawnObjects`
  (for _array_element (`self.ItemsToSpawn`)
    (bind _returnvalue (`|SpawnActorFromClass` (`/Game/MiniGames/Blueprints/ObjectToSpawn.Item` _array_element) (`KismetMathLibrary.Conv_VectorToTransform` (`self.K2_GetActorLocation` _array_element)) "Undefined" "MultiplyWithRoot" null null))
    (`KismetArrayLibrary.Array_Add` (`self.Items`) _returnvalue)))

(fn `UserConstructionScript`)