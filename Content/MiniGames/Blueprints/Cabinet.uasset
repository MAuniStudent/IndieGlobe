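; Cabinet is an interactable mini-game actor that checks whether the player's selected item belongs in it.
; On Interact, it compares the MiniGameCharacter's selected item ID to its own, then spawns green or red Niagara feedback and raises or lowers the score.
; A wrong timed item also triggers the fail screen.
; Either result calls TaskChange on the item and hides the UI time text.
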(event `/Game/MiniGames/Blueprints/InteractInterface.Interact`
  (params (Object :type "Object Object Reference"))
  (bind _returnvalue (`self.K2_GetActorLocation`))
  (bind _asmini_game_character (cast `/Game/MiniGames/Blueprints/MiniGameCharacter` Object))
  (bind _newparam (`/Game/MiniGames/Blueprints/MiniGameCharacter.GetSelectedItem` _asmini_game_character))
  (if (`KismetSystemLibrary.IsValid` _newparam)
    (if (== (`/Game/MiniGames/Blueprints/Item.ID` _newparam) (`self.ID`))
      (`NiagaraFunctionLibrary.SpawnSystemAtLocation` "/Game/VFX/System/NS_floatGreen.NS_floatGreen" _returnvalue)
      (`/Game/MiniGames/Blueprints/MiniGameCharacter.UpdateScore` _asmini_game_character 10)
      (else
        (`NiagaraFunctionLibrary.SpawnSystemAtLocation` "/Game/VFX/System/NS_floatRed.NS_floatRed" _returnvalue)
        (`/Game/MiniGames/Blueprints/MiniGameCharacter.UpdateScore` _asmini_game_character -10)
        (if (`/Game/MiniGames/Blueprints/Item.isTimed` _newparam)
          (`/Game/MiniGames/Blueprints/MiniGameCharacter.Fail Screen` _asmini_game_character))))
    (`/Game/MiniGames/Blueprints/Item.TaskChange` _newparam)
    (`/Game/MiniGames/Blueprints/MiniGameUI.TimeTextHidden` (`/Game/MiniGames/Blueprints/MiniGameCharacter.UI` _asmini_game_character))))

(fn `UserConstructionScript`)