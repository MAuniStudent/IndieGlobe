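; Timed special "Yellow" mini-game item, a child pickup that sets its own ID and name and spawns a Niagara effect above itself.
; Tick uses a Delay as a one-second countdown on TimeLeft, calling FailScreen on the MiniGameCharacter when time runs out.
; It also pushes the remaining time each tick to the UI slot matching its TaskNum.
; Pickup runs the parent logic, then destroys the effect.
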(event `self.ReceiveBeginPlay`
  (bind (_returnvalue_x _returnvalue_y _returnvalue_z) (`KismetMathLibrary.BreakVector` (`self.K2_GetActorLocation` self)))
  (`parent.ReceiveBeginPlay`)
  (set `self.ID` 3)
  (set `self.Name` "Yellow")
  (set `self.isTimed` true)
  (bind _returnvalue (`NiagaraFunctionLibrary.SpawnSystemAtLocation` "/Game/VFX/System/NS_Special.NS_Special" (`KismetMathLibrary.MakeVector` _returnvalue_x _returnvalue_y (+ _returnvalue_z 50.0))))
  (set `self.VFX` _returnvalue))

(event `self.ReceiveActorBeginOverlap`
  (params (OtherActor :type "Actor Object Reference"))
  (`parent.ReceiveActorBeginOverlap` OtherActor))

(event `self.ReceiveTick`
  (params (DeltaSeconds :type "Float (single-precision)"))
  (bind _timeleft (`self.TimeLeft`))
  (bind _tasknum (`self.TaskNum`))
  (bind _ui (`self.UI`))
  (bind _returnvalue (`KismetTextLibrary.Conv_IntToText` _timeleft))
  (`parent.ReceiveTick` DeltaSeconds)
  (`|ExecutionSequence`
    (:`then_0`
      (`KismetSystemLibrary.Delay` 1.0)
      (set `self.TimeLeft` (- _timeleft 1))
      (if (<= (`self.TimeLeft`) 0)
        (bind _returnvalue_2 (`GameplayStatics.GetActorOfClass` "/Game/MiniGames/Blueprints/MiniGameCharacter.MiniGameCharacter_C"))
        (`/Game/MiniGames/Blueprints/MiniGameCharacter.Fail Screen` _returnvalue_2)))
    (:`then_1`
      (if (== (`self.TaskNum`) 1)
        (`/Game/MiniGames/Blueprints/MiniGameUI.UpdateTask1Time` _ui _returnvalue)
        (elif (== _tasknum 2)
          (`/Game/MiniGames/Blueprints/MiniGameUI.UpdateTask2Time` _ui _returnvalue)
          (elif (== _tasknum 3)
            (`/Game/MiniGames/Blueprints/MiniGameUI.UpdateTask3Time` _ui _returnvalue)))))))

(fn `onPickUp`
  (`parent.onPickUp`)
  (`ActorComponent.K2_DestroyComponent` (`self.VFX`)))

(fn `UserConstructionScript`
  (`parent.UserConstructionScript`))